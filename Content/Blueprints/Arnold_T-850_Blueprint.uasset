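; Arnold_T-850_Blueprint is a damageable actor, apparently a Terminator-style target, that can be shot or run over.
; Its mesh hit event destroys any FirstPersonProjectile that strikes it and calls Bullethit, which lowers HP by one and destroys the actor at zero.
; A hit from a Sedan destroys it instantly.
; An explosion sound node is present but disconnected, so it never plays.
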(event `self.StaticMeshComponent.OnComponentHit`
  (params (HitComponent :type "PrimitiveComponent Object Reference") (OtherActor :type "Actor Object Reference") (OtherComp :type "PrimitiveComponent Object Reference") (NormalImpulse :type "Vector Structure") (Hit :type "HitResult Structure (by ref)"))
  (bind _asfirst_person_projectile (cast `/Game/FirstPersonBP/Blueprints/FirstPersonProjectile` OtherActor)
    (:`then`
      (`self.K2_DestroyActor` _asfirst_person_projectile)
      (`self.bullethit`))
    (:`CastFailed`
      (cast `/Game/VehicleBP/Sedan/Sedan` OtherActor)
      (`self.K2_DestroyActor`))))

(fn `bullethit`
  (bind _output_get (set `self.HP` (- (`self.HP`) 1)))
  (if (<= _output_get 0)
    (`self.K2_DestroyActor`)))

(fn `UserConstructionScript`)